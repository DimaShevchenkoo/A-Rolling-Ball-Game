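; Game mode for a rolling ball game that sets up the level's cubes and tracks the win condition.
; On BeginPlay it shows the WB_UserInterface widget, then spawns random numbers of base and cleaner cubes at random positions, counting each type.
; Tick polls all actors tagged "Marked" and sets Won once their count reaches the combined base and cleaner total.
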(event EventBeginPlay
  (bind _returnvalue (UserInterface|CreateWidget "/Game/Blueprints/WB_UserInterface.WB_UserInterface_C"))
  (UserInterface|Viewport|AddtoViewport _returnvalue 0)
  (CallFunction|SpawnBaseCube)
  (CallFunction|SpawnCleanerCube))

(event EventTick
  (params (DeltaSeconds :type Float%20%28single-precision%29))
  (bind _outactors (Actor|GetAllActorswithTag "Marked"))
  (for (_ _array_index) _outactors
    (if (== _array_index (- (+ (Variables|Default|GetBase%20Amount) (Variables|Default|GetCleaner%20Amount)) 1))
      (Variables|Default|SetWon? true))))

(fn ConstructionScript)

(fn SpawnBaseCube
  (for _index (range 0 (Math|Random|RandomIntegerinRange 10 15))
    (bind _result (Math|Integer|IncrementInt (Variables|Default|GetBase%20Amount))
      (:%20%20
        (Variables|Default|SetBase%20Amount _result)
        (bind _output_get (Variables|Default|SetNewVar (Math|Vector|MakeVector (Math|Conversions|ToFloat(Integer) (Math|Random|RandomIntegerinRange 55 1760)) (Math|Conversions|ToFloat(Integer) (Math|Random|RandomIntegerinRange 150 1760)) 4e+01)))
        (Game|SpawnActorfromClass "/Game/Blueprints/BP_CubeBase.BP_CubeBase_C" (Math|Transform|MakeTransform _output_get) "AdjustIfPossibleButAlwaysSpawn" "MultiplyWithRoot" 0 0)))))

(fn SpawnCleanerCube
  (for _index (range 0 (Math|Random|RandomIntegerinRange 4 7))
    (bind _result (Math|Integer|IncrementInt (Variables|Default|GetCleaner%20Amount))
      (:%20%20
        (Variables|Default|SetCleaner%20Amount _result)
        (bind _output_get (Variables|Default|SetNewVar (Math|Vector|MakeVector (Math|Conversions|ToFloat(Integer) (Math|Random|RandomIntegerinRange 55 1760)) (Math|Conversions|ToFloat(Integer) (Math|Random|RandomIntegerinRange 150 1760)) 4e+01)))
        (Game|SpawnActorfromClass "/Game/Blueprints/BP_CubeCleaner.BP_CubeCleaner_C" (Math|Transform|MakeTransform _output_get) "AdjustIfPossibleButAlwaysSpawn" "MultiplyWithRoot" 0 0)))))